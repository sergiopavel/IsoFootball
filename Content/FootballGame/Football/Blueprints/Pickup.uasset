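; Collectible target pickup for the top-down football game that also ends the run if the player passes it.
; It spins its static mesh every tick.
; Overlapping the Box with the TopDownCharacter increments the game mode's Pick count, plays a 2D sound and destroys the pickup.
; Two side triggers, EndGame1 and EndGame2, instead call the character's Gameover and show the mouse cursor.
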(event OnComponentBeginOverlap(Box)
  (params (OverlappedComponent :type Primitive%20Component%20Object%20Reference) (OtherActor :type Actor%20Object%20Reference) (OtherComp :type Primitive%20Component%20Object%20Reference) (OtherBodyIndex :type Integer) (bFromSweep :type Boolean) (SweepResult :type Hit%20Result%20Structure%20%28by%20ref%29))
  ;[1 1 1] Picking and counting targets
  (Utilities|Casting|CastToTopDownCharacter OtherActor)
  (bind _astop_down_game_mode (Utilities|Casting|CastToTopDownGameMode (Game|GetGameMode)))
  (Math|Integer|IncrementInt (Variables|/Game/FootballGame/Character_RulesBP/TopDownGameMode.TopDownGameMode_C|Getpick _astop_down_game_mode)
    (:%20%20
      (Audio|SpawnSound2D "/Game/FootballGame/Football/PitchComponents/Robot_blip-Marianne_Gagnon-120342607.Robot_blip-Marianne_Gagnon-120342607" 1.0 1.0 0.0 0)
      (Actor|DestroyActor))))

(event OnComponentBeginOverlap(EndGame1)
  (params (OverlappedComponent :type Primitive%20Component%20Object%20Reference) (OtherActor :type Actor%20Object%20Reference) (OtherComp :type Primitive%20Component%20Object%20Reference) (OtherBodyIndex :type Integer) (bFromSweep :type Boolean) (SweepResult :type Hit%20Result%20Structure%20%28by%20ref%29))
  ;[1 1 1] GameOver if pass a target
  (bind _astop_down_character (Utilities|Casting|CastToTopDownCharacter OtherActor))
  (Default|Gameover _astop_down_character)
  (Variables|/Script/Engine.PlayerController|SetbShowMouseCursor (Game|GetPlayerController 0) true))

(event OnComponentBeginOverlap(EndGame2)
  (params (OverlappedComponent :type Primitive%20Component%20Object%20Reference) (OtherActor :type Actor%20Object%20Reference) (OtherComp :type Primitive%20Component%20Object%20Reference) (OtherBodyIndex :type Integer) (bFromSweep :type Boolean) (SweepResult :type Hit%20Result%20Structure%20%28by%20ref%29))
  ;[1 1 1] GameOver if pass a target
  (bind _astop_down_character (Utilities|Casting|CastToTopDownCharacter OtherActor))
  (Default|Gameover _astop_down_character)
  (Variables|/Script/Engine.PlayerController|SetbShowMouseCursor (Game|GetPlayerController 0) true))

(event EventTick
  (params (DeltaSeconds :type Float%20%28single-precision%29))
  ;[1 1 1] Rotation Animation for Target
  (Transformation|AddRelativeRotation (Variables|Default|GetStaticMesh) (Math|Rotator|MakeRotator 0.0 0.0 (* DeltaSeconds 1.5e+02)) false false))

(fn ConstructionScript)