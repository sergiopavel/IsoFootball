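; Endless-runner pitch segment for a football game that chains new field pieces as the player crosses it.
; On begin play it has an even chance of spawning a pickup on one of four lanes.
; When the player overlaps its box, the game mode counts segments and spawns the next, adding score, raising walk speed within a clamp, then destroying this piece.
; At the length limit it spawns the final pitch and stops player movement.
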(event OnComponentBeginOverlap(Box)
  (params (OverlappedComponent :type Primitive%20Component%20Object%20Reference) (OtherActor :type Actor%20Object%20Reference) (OtherComp :type Primitive%20Component%20Object%20Reference) (OtherBodyIndex :type Integer) (bFromSweep :type Boolean) (SweepResult :type Hit%20Result%20Structure%20%28by%20ref%29))
  ;[1 1 1] Spawn a new piece of field at the and of each untill passing it
  (Utilities|Casting|CastToTopDownCharacter OtherActor)
  ;;[1 1 1] Counting how many pieces passed
  (bind _astop_down_game_mode (Utilities|Casting|CastToTopDownGameMode (Game|GetGameMode)))
  (bind _output_get (Variables|/Game/FootballGame/Character_RulesBP/TopDownGameMode.TopDownGameMode_C|Settime _astop_down_game_mode (+ (Variables|/Game/FootballGame/Character_RulesBP/TopDownGameMode.TopDownGameMode_C|Gettime _astop_down_game_mode) 1)))
  (if (== _output_get 50)
    ;;[1 1 1] Spawning last piece of football pitch if reaching maximum of level lenght
    (bind _astop_down_game_mode_2 (Utilities|Casting|CastToTopDownGameMode (Game|GetGameMode)))
    (Default|SpawnLastPitch _astop_down_game_mode_2)
    (Utilities|FlowControl|Delay 2.0)
    (bind _astop_down_character (Utilities|Casting|CastToTopDownCharacter (Game|GetPlayerCharacter 0)))
    (Pawn|Components|CharacterMovement|DisableMovement (Variables|/Script/Engine.Character|GetCharacterMovement _astop_down_character))
    (else
      (Default|Spawn _astop_down_game_mode)
      (bind _astop_down_game_mode_3 (Utilities|Casting|CastToTopDownGameMode (Game|GetGameMode)))
      (Variables|/Game/FootballGame/Character_RulesBP/TopDownGameMode.TopDownGameMode_C|Setscore _astop_down_game_mode_3 (+ (Variables|/Game/FootballGame/Character_RulesBP/TopDownGameMode.TopDownGameMode_C|Getscore _astop_down_game_mode_3) 1))
      ;;[1 1 1] Increasing speed piece of field by piece
      (bind _astop_down_character_2 (Utilities|Casting|CastToTopDownCharacter (Game|GetPlayerCharacter 0)))
      (Variables|/Script/Engine.CharacterMovementComponent|SetMaxWalkSpeed (Variables|/Script/Engine.Character|GetCharacterMovement _astop_down_character_2) (Math|Float|Clamp(Float) (* (Variables|/Script/Engine.CharacterMovementComponent|GetMaxWalkSpeed (Variables|/Script/Engine.Character|GetCharacterMovement _astop_down_character_2)) 1.02) 6e+02 2e+03))
      (Utilities|FlowControl|Delay 5.0)
      (Actor|DestroyActor))))

(event EventBeginPlay
  ;[1 1 1] Spawn targets
  (CallFunction|Randomtarget))

(fn ConstructionScript)

(fn Randomtarget
  ;[1 1 1] Spawn a target
  (switch int (Math|Random|RandomIntegerinRange 0 1)
    (:1
      (Game|SpawnActorfromClass "/Game/FootballGame/Football/Blueprints/Pickup.Pickup_C" (Transformation|GetWorldTransform (Utilities|Array|Get(acopy) (Utilities|Array|MakeArray (Variables|Default|Getl1) (Variables|Default|Getl2) (Variables|Default|Getl3) (Variables|Default|Getl4)) (Math|Random|RandomIntegerinRange 0 3))) "Undefined" 0 0))))